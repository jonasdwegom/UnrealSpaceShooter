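; BP_Player is the player-controlled shooter, sliding sideways along the world Y axis within fixed bounds.
; Fire input spawns a BP_Shoot projectile at the PointShooter component.
; A BP_Enemy overlapping its Box is destroyed and calls DecLife on the GS_Jogo game state.
; It creates the WB_HUD widget on BeginPlay and refreshes score and life text from GS_Jogo every Tick.
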(event OnComponentBeginOverlap(Box)
  (params (OverlappedComponent :type Primitive%20Component%20Object%20Reference) (OtherActor :type Actor%20Object%20Reference) (OtherComp :type Primitive%20Component%20Object%20Reference) (OtherBodyIndex :type Integer) (bFromSweep :type Boolean) (SweepResult :type Hit%20Result%20Structure%20%28by%20ref%29))
  ;[1 1 1] Destroi o inimigo e decrementa a vida do player
  (Utilities|Casting|CastToBP_Enemy OtherActor)
  (bind _asgs_jogo (Utilities|Casting|CastToGS_Jogo (Game|GetGameState)))
  (Default|DecLife _asgs_jogo)
  (Actor|DestroyActor OtherActor))

(event Collision|EventActorBeginOverlap
  (params (OtherActor :type Actor%20Object%20Reference)))

(event EventBeginPlay
  ;[1 1 1] Cria a widget (HUD) e define como viewport (Exibe na tela)
  (bind _returnvalue (UserInterface|CreateWidget "/Game/Interface/WB_HUD.WB_HUD_C"))
  (bind _output_get (Variables|Default|SetHUD _returnvalue))
  (UserInterface|Viewport|AddtoViewport _output_get 0))

(event EventTick
  (params (DeltaSeconds :type Float%20%28single-precision%29))
  (bind _hud (Variables|Default|GetHUD))
  (bind _asgs_jogo (Utilities|Casting|CastToGS_Jogo (Game|GetGameState)))
  (Rendering|Components|TextRender|SetText (Variables|/Game/Interface/WB_HUD.WB_HUD_C|GettxtScore _hud) (Utilities|Text|ToText(Float) (Variables|/Game/Blueprints/GS_Jogo.GS_Jogo_C|GetScore _asgs_jogo) "HalfToEven"))
  (Rendering|Components|TextRender|SetText (Variables|/Game/Interface/WB_HUD.WB_HUD_C|GettxtLife _hud) (Utilities|Text|ToText(Integer) (Variables|/Game/Blueprints/GS_Jogo.GS_Jogo_C|GetLife _asgs_jogo))))

(event Input|ActionEvents|InputActionFire
  (params (Key :type Key%20Structure))
  ;[1 1 1] Cria o tiro
  (:Pressed
    (Game|SpawnActorfromClass "/Game/Blueprints/BP_Shoot.BP_Shoot_C" (Math|Transform|MakeTransform (Transformation|GetWorldLocation (Variables|Default|GetPointShooter)) "90.000000, 0, 0") "Undefined" 0 0)))

(event Input|AxisEvents|InputAxisMoveHorizontal
  (params (AxisValue :type Float%20%28single-precision%29))
  (bind _returnvalue (Transformation|GetActorLocation))
  (bind _speedy (Variables|Default|GetSpeedy))
  (bind _returnvalue_2 (* AxisValue _speedy))
  (bind _returnvalue_3 (+ _returnvalue_2 (.y _returnvalue)))
  ;[1 1 1] Movimenta o player
  (if (and (>= _returnvalue_3 -2e+03) (<= _returnvalue_3 2e+03))
    (Transformation|SetActorLocation (Math|Vector|MakeVector (.x _returnvalue) _returnvalue_3 (.z _returnvalue)) false false)))

(fn ConstructionScript)